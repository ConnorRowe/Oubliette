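; BP_Spell_Projectile is a spell projectile that deals radial damage on impact.
; Init passes damage, element, speed and double-explode chance to its parent, then sets movement speed.
; Hits on anything except the instigator apply full damage, with a chance of doubled radius.
; Unless it hit another spell projectile, it pushes physics objects, notifies the caster, plays explosion effects, hides, disables collision and destroys itself after a delay.
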(event `self.initProjectile`
  (params (CalcedDamage :type "Float (single-precision)") (Element :type "DamageType Class Reference") (ProjectileSpeed :type "Float (single-precision)") (DoubleExplodeChance :type "Float (single-precision)"))
  (bind _projectile (`self.Projectile`))
  (`parent.initProjectile` CalcedDamage Element ProjectileSpeed DoubleExplodeChance)
  (set `self.doubleExplodeChance` DoubleExplodeChance)
  (bind _output_get (set `self.projectileSpeed` ProjectileSpeed))
  (set `ProjectileMovementComponent.InitialSpeed` _output_get _projectile)
  (set `ProjectileMovementComponent.MaxSpeed` _output_get _projectile))

(event `self.ReceiveHit`
  (params (MyComp :type "PrimitiveComponent Object Reference") (Other :type "Actor Object Reference") (OtherComp :type "PrimitiveComponent Object Reference") (bSelfMoved :type Boolean) (HitLocation :type "Vector Structure") (HitNormal :type "Vector Structure") (NormalImpulse :type "Vector Structure") (Hit :type "HitResult Structure (by ref)"))
  (bind _returnvalue (`self.GetInstigator`))
  ;[1 1 1] Hit Logic
  (if (not (== Other (`self.GetInstigator`)))
    (`GameplayStatics.ApplyRadialDamage` (`self.spellDamage`) HitLocation (select `bool` (< (`KismetMathLibrary.RandomFloat`) (`self.doubleExplodeChance`)) :`false` 30.0 :`true` 60.0 :!type "Float (single-precision)") (`self.damageType`) (`|MakeArray` _returnvalue :!type "Actor Object Reference") _returnvalue null true "ECC_Camera")
    (cast `/Game/Blueprint/Spells/Projectile/BP_Spell_Projectile` Other
      (:`CastFailed`
        (if (!= Other (`self.GetInstigator`))
          (if (`SceneComponent.IsSimulatingPhysics` OtherComp "None")
            (`PrimitiveComponent.AddImpulseAtLocation` OtherComp (* (`self.GetVelocity`) 100.0) (`self.K2_GetActorLocation`) "None"))
          (`/Game/Blueprint/Character/BP_Oubliette_Character.HasHitSomething` (cast `/Game/Blueprint/Character/BP_Oubliette_Character` (`self.GetInstigator`) :!pure true))
          (`GameplayStatics.SpawnEmitterAtLocation` (`self.DestroyEmitter`) HitLocation)
          (set `self.isDestroyed` true)
          (`SceneComponent.SetVisibility` (`self.Sphere`) false false)
          (`ParticleSystemComponent.SetVectorParameter` (`self.ParticleSystem`) "ChargeV" (0.0 0.0 0.0))
          (`GameplayStatics.PlaySoundAtLocation` "/Game/Sound/Spell_Explosion_Cue.Spell_Explosion_Cue" HitLocation (struct) 1.0 1.0 0.0 null null null)
          (`PrimitiveComponent.SetCollisionResponseToAllChannels` (`self.CollisionComponent`) "ECR_Ignore")
          (`PrimitiveComponent.SetCollisionResponseToAllChannels` (`self.Sphere`) "ECR_Ignore")
          (`KismetSystemLibrary.Delay` 1.0)
          (`self.K2_DestroyActor`) ; Then destroy this projectile
        )))))

(fn `UserConstructionScript`)