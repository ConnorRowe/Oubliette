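; BP_Spell_Channel is a channeled spell actor that repeatedly damages BP_Enemy actors at its location.
; A looping timer runs DamageTick, which does a small stationary box trace and scales Damage by the tick interval, making it damage per second.
; Enemy hits notify the Oubliette_Character instigator, while any hit fires the "Main" event on PDamage, whose particle template is set in the construction script.
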(event `self.ReceiveBeginPlay`
  (`KismetSystemLibrary.K2_SetTimer` null "DamageTick" 0.2 true))

(fn `DamageTick`
  (locals (hasHit :type Boolean :default false))
  (bind _returnvalue (`self.K2_GetActorLocation`))
  (bind (_outhits _returnvalue_2) (`KismetSystemLibrary.BoxTraceMultiForObjects` :`Start` _returnvalue :`End` _returnvalue :`HalfSize` (10.0 10.0 10.0) :`ObjectTypes` (`|MakeArray` "ObjectTypeQuery1" "ObjectTypeQuery2" "ObjectTypeQuery3" "ObjectTypeQuery4" :!type "EObjectTypeQuery Enum") :`DrawTime` 0.1))
  (set `local.hasHit` _returnvalue_2)
  (for _array_element _outhits
    (bind _asbp_enemy (cast `/Game/Blueprint/BP_Enemy` (`.HitActor` (`GameplayStatics.BreakHitResult` _array_element))))
    (`GameplayStatics.ApplyDamage` _asbp_enemy (* (`self.Damage`) 0.2) (`self.GetInstigatorController`) (`self.GetInstigator`) (`self.DamageType`))
    (`ParticleSystemComponent.GenerateParticleEvent` (`self.P_Damage`) "Main" 0.0 (0.0 0.0 0.0) (0.0 0.0 0.0) (0.0 0.0 0.0))
    (`/Game/Blueprint/Character/Oubliette_Character.HasHitSomething` (cast `/Game/Blueprint/Character/Oubliette_Character` (`self.Instigator`) :!pure true)))
  (if (`local.hasHit`)
    (`ParticleSystemComponent.GenerateParticleEvent` (`self.P_Damage`) "Main" 0.0 (0.0 0.0 0.0) (0.0 0.0 0.0) (0.0 0.0 0.0))))

(fn `UserConstructionScript`
  (`ParticleSystemComponent.SetTemplate` (`self.P_Damage`) (`self.DamageParticle`)))