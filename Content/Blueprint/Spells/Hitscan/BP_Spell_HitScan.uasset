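; Hitscan spell actor that damages pawns around its location and destroys itself two seconds after spawning.
; DealDamage, not called within this Blueprint, applies full radial damage in a small radius, ignoring the instigator, then sphere-traces a wider radius for pawns.
; BP_Enemy hits take additional direct damage, with AlreadyDamaged skipping only the most recently damaged actor.
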(event `self.ReceiveBeginPlay`
  (`KismetSystemLibrary.Delay` 2.0)
  (`self.K2_DestroyActor`))

(fn `DealDamage`
  (locals (IgnoredActors :type "Array of Actor Object Reference") (AlreadyDamaged :type "Actor Object Reference"))
  (bind _returnvalue (`self.K2_GetActorLocation`))
  (bind _returnvalue_2 (`self.GetInstigator`))
  (`GameplayStatics.ApplyRadialDamage` (`self.spellDamage`) _returnvalue 10.0 (`self.damageType`) (`|MakeArray` _returnvalue_2 :!type "Actor Object Reference") _returnvalue_2 null true)
  (bind _outhits (`KismetSystemLibrary.SphereTraceMultiForObjects` _returnvalue (+ _returnvalue (0.0 0.0 1.0)) 50.0 (`|MakeArray` "ObjectTypeQuery3" :!type "EObjectTypeQuery Enum")))
  (for _array_element _outhits
    (bind (_bblockinghit _binitialoverlap _time _distance _location _impactpoint _normal _impactnormal _physmat _hitactor) (`GameplayStatics.BreakHitResult` _array_element))
    (if _bblockinghit
      (bind _asbp_enemy (cast `/Game/Blueprint/AI/Enemies/BP_Enemy` _hitactor))
      (if (not (== _hitactor (`local.AlreadyDamaged`)))
        (`GameplayStatics.ApplyDamage` _asbp_enemy (`self.spellDamage`) (`self.GetInstigatorController`) (`self.GetInstigator`) (`self.damageType`))
        (set `local.AlreadyDamaged` _hitactor)))))

(fn `UserConstructionScript`)