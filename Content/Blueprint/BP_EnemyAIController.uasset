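; BP_EnemyAIController is an enemy AI controller that runs the BT_Hopping behavior tree on its pawn.
; On BeginPlay it sets up the BB_Follow blackboard, then after a short delay stores the pawn's location as HomeLocation and starts the tree.
; Perception updates log the updated actors' names and save the first one as TargetActor, which this graph does not write to the blackboard.
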(event `self.AIPerception.OnPerceptionUpdated`
  (params (UpdatedActors :type "Array of Actor Object Reference (by ref)"))
  (bind _updatedactors (`self.UpdatedActors`))
  (for _array_element UpdatedActors
    (set `self.UpdatedActors` (`KismetStringLibrary.Concat_StrStr` _updatedactors (`KismetSystemLibrary.GetDisplayName` _array_element) ", ")))
  (`KismetSystemLibrary.PrintString` _updatedactors false)
  (set `self.UpdatedActors` "Updated Actors: ")
  (set `self.TargetActor` (`|GetArrayItem` UpdatedActors)))

(event `self.ReceiveBeginPlay`
  (bind _blackboardcomponent (`self.UseBlackboard` "/Game/Blueprint/AI/BB_Follow.BB_Follow"))
  (set `self.EnemyBlackboard` _blackboardcomponent)
  (`KismetSystemLibrary.Delay` 0.2)
  (`BlackboardComponent.SetValueAsVector` (`self.EnemyBlackboard`) (`self.Home Location`) (`self.K2_GetActorLocation` (`self.K2_GetPawn`)))
  (`self.RunBehaviorTree` "/Game/Blueprint/AI/BT_Hopping.BT_Hopping"))

(fn `UserConstructionScript`)