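; Game mode for Oubliette that loads item data from DataTables and generates random items.
; On BeginPlay it fills a five-rarity general chest pool, a flat starter pool, and prefix and suffix affix arrays.
; GenerateRandomItem draws from a rarity-tiered pool with unweighted tier odds, replacing "rand" prefix or suffix placeholders with random affixes and appending their stats.
; A GetDataTableLength helper counts rows by probing sequential NewRow names.
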(event `self.ReceiveBeginPlay`
  (`self.LoadItemPool` "/Game/Blueprint/Items/ItemPool_GeneralChest_Common.ItemPool_GeneralChest_Common" "/Game/Blueprint/Items/ItemPool_GeneralChest_Uncommon.ItemPool_GeneralChest_Uncommon" "/Game/Blueprint/Items/ItemPool_GeneralChest_Rare.ItemPool_GeneralChest_Rare" "/Game/Blueprint/Items/ItemPool_GeneralChest_Epic.ItemPool_GeneralChest_Epic" "/Game/Blueprint/Items/ItemPool_GeneralChest_Legendary.ItemPool_GeneralChest_Legendary" (`self.ItemPool_GeneralChest`))
  (`self.LoadSingleItemPool` "/Game/Blueprint/Items/ItemPool_Starter.ItemPool_Starter" (`self.ItemPool_Starter`))
  (`self.LoadAffixes` "/Game/Blueprint/Items/ItemPrefixes.ItemPrefixes" (`self.ItemPrefixes`))
  (`self.LoadAffixes` "/Game/Blueprint/Items/ItemSuffixes.ItemSuffixes" (`self.ItemSuffixes`)))

(fn `GenerateRandomItem`
  (params (ItemPool :type "ItemPoolStruct Structure"))
  (returns (Item :type "ItemStruct Structure"))
  (locals (ReturnItem :type "ItemStruct Structure") (TempStats :type "Array of StatStruct Structure") (TempAffix :type "ItemAffixStruct Structure"))
  (bind (_common _uncommon _rare _epic _legendary) (break `ItemPoolStruct` ItemPool))
  (bind _itemprefixes (`self.ItemPrefixes`))
  (bind _itemsuffixes (`self.ItemSuffixes`))
  (bind (_rarity _prefix _name _suffix) (break `ItemStruct` (`local.ReturnItem`)))
  (bind _returnvalue (select `int` (`KismetMathLibrary.RandomIntegerInRange` 0 4) :`0` _common :`1` _uncommon :`2` _rare :`3` _epic :`4` _legendary))
  (set `local.ReturnItem` (`|GetArrayItem` _returnvalue (`KismetMathLibrary.RandomIntegerInRange` 0 (- (`KismetArrayLibrary.Array_Length` _returnvalue) 1))))
  (if (`KismetTextLibrary.EqualEqual_TextText` _prefix "rand")
    (bind _output_get (set `local.TempStats` (`.Stats` (break `ItemStruct` (`local.ReturnItem`)))))
    (bind _output_get_2 (set `local.TempAffix` (`|GetArrayItem` _itemprefixes (`KismetMathLibrary.RandomIntegerInRange` 0 (- (`KismetArrayLibrary.Array_Length` _itemprefixes) 1)))))
    (`KismetArrayLibrary.Array_Append` _output_get (`.Stats` (break `ItemAffixStruct` _output_get_2)))
    (setmembers `ItemStruct` :`StructRef` (`local.ReturnItem`) :`Prefix` (`KismetTextLibrary.Conv_NameToText` (break `ItemAffixStruct` _output_get_2)) :`Stats` (`local.TempStats`)))
  (if (`KismetTextLibrary.EqualEqual_TextText` _suffix "rand")
    (bind _output_get_3 (set `local.TempAffix` (`|GetArrayItem` _itemsuffixes (`KismetMathLibrary.RandomIntegerInRange` 0 (- (`KismetArrayLibrary.Array_Length` _itemsuffixes) 1)))))
    (bind _output_get_4 (set `local.TempStats` (`.Stats` (break `ItemStruct` (`local.ReturnItem`)))))
    (`KismetArrayLibrary.Array_Append` _output_get_4 (`.Stats` (break `ItemAffixStruct` _output_get_3)))
    (setmembers `ItemStruct` :`StructRef` (`local.ReturnItem`) :`Suffix` (`KismetTextLibrary.Conv_NameToText` (break `ItemAffixStruct` _output_get_3)) :`Stats` (`local.TempStats`)))
  (return (`local.ReturnItem`)))

(fn `GetDataTableLength`
  (params (Table :type "DataTable Object Reference"))
  (returns (Length :type Integer))
  (locals (HasEndBeenFound :type Boolean) (iteration :type Integer))
  (while (not (`local.HasEndBeenFound`))
    (bind _returnvalue (`DataTableFunctionLibrary.DoesDataTableRowExist` Table (`KismetStringLibrary.Conv_StringToName` (select `bool` (> (`local.iteration`) 0) :`false` "NewRow" :`true` (`KismetStringLibrary.BuildString_Int` "" "NewRow_" (- (`local.iteration`) 1))))))
    (set `local.HasEndBeenFound` (not _returnvalue))
    (`/Engine/EditorBlueprintResources/StandardMacros.IncrementInt` (`local.iteration`)))
  (return (- (`local.iteration`) 1)))

(fn `LoadAffixes`
  (params (AffixTable :type "DataTable Object Reference") (AffixArray :type "Array of ItemAffixStruct Structure (by ref)"))
  (bind _outrownames (`DataTableFunctionLibrary.GetDataTableRowNames` AffixTable))
  (for _array_element _outrownames
    (bind _returnvalue (`|GetDataTableRow` AffixTable _array_element)
      (:`then`
        (`KismetArrayLibrary.Array_Add` AffixArray _returnvalue)))))

(fn `LoadItemPool`
  (params (`Common Item Pool` :type "DataTable Object Reference") (`Uncommon Item Pool` :type "DataTable Object Reference") (`Rare Item Pool` :type "DataTable Object Reference") (`Epic Item Pool` :type "DataTable Object Reference") (`Legendary Item Pool` :type "DataTable Object Reference") (`Target Item Pool` :type "ItemPoolStruct Structure (by ref)"))
  (bind (_common _uncommon _rare _epic _legendary) (break `ItemPoolStruct` `Target Item Pool`))
  (for _index (range 5)
    (bind _returnvalue (select `int` _index :`0` `Common Item Pool` :`1` `Uncommon Item Pool` :`2` `Rare Item Pool` :`3` `Epic Item Pool` :`4` `Legendary Item Pool`))
    (bind _outrownames (`DataTableFunctionLibrary.GetDataTableRowNames` _returnvalue))
    (for _array_element _outrownames
      (bind _returnvalue_2 (`|GetDataTableRow` _returnvalue _array_element)
        (:`then`
          (bind (_id _rarity _prefix _name _suffix _effect _effectmagnitude _stats _flavourtext _itemtype _icon _rcolour _gcolour _bcolour) (break `ItemDataTableStruct` _returnvalue_2))
          (`KismetArrayLibrary.Array_Add` (select `int` _index :`0` _common :`1` _uncommon :`2` _rare :`3` _epic :`4` _legendary) (make `ItemStruct` _rarity (`KismetTextLibrary.Conv_StringToText` _prefix) (`KismetTextLibrary.Conv_StringToText` _name) (`KismetTextLibrary.Conv_StringToText` _suffix) _effect _effectmagnitude _stats _flavourtext _itemtype _icon _rcolour _gcolour _bcolour)))))))

(fn `LoadSingleItemPool`
  (params (`Item Pool` :type "DataTable Object Reference") (`Target Item Pool` :type "Array of ItemStruct Structure (by ref)"))
  (bind _outrownames (`DataTableFunctionLibrary.GetDataTableRowNames` `Item Pool`))
  (for _array_element _outrownames
    (bind _returnvalue (`|GetDataTableRow` `Item Pool` _array_element)
      (:`then`
        (bind (_id _rarity _prefix _name _suffix _effect _effectmagnitude _stats _flavourtext _itemtype _icon _rcolour _gcolour _bcolour) (break `ItemDataTableStruct` _returnvalue))
        (`KismetArrayLibrary.Array_Add` `Target Item Pool` (make `ItemStruct` _rarity (`KismetTextLibrary.Conv_StringToText` _prefix) (`KismetTextLibrary.Conv_StringToText` _name) (`KismetTextLibrary.Conv_StringToText` _suffix) _effect _effectmagnitude _stats _flavourtext _itemtype _icon _rcolour _gcolour _bcolour))))))

(fn `UserConstructionScript`)