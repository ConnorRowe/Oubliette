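; BP_Room_New is a dungeon room actor that tracks whether the player is in combat inside it.
; A looping timer started on BeginPlay scans RoomBoxVolume overlaps for the player character and living enemies.
; When the player is present, it sets IsInCombat on BP_GameModeOubliette according to whether a living enemy shares the room.
; Radial damage adds a strong radial force to the hit component at the impact point.
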(event `self.ReceiveBeginPlay`
  (`KismetSystemLibrary.K2_SetTimer` null "CheckForCombat" 0.5 true))

(event `self.ReceiveRadialDamage`
  (params (DamageReceived :type "Float (single-precision)") (DamageType :type "DamageType Object Reference") (Origin :type "Vector Structure") (HitInfo :type "HitResult Structure (by ref)") (InstigatedBy :type "Controller Object Reference") (DamageCauser :type "Actor Object Reference"))
  (bind (_bblockinghit _binitialoverlap _time _distance _location _impactpoint _normal _impactnormal _physmat _hitactor _hitcomponent) (`GameplayStatics.BreakHitResult` HitInfo))
  (`PrimitiveComponent.AddRadialForce` _hitcomponent _impactpoint 100.0 2000000.0 "RIF_Linear" false))

(fn `CheckForCombat`
  (locals (foundEnemy :type Boolean) (foundPlayer :type Boolean))
  (bind _foundplayer (`local.foundPlayer`))
  (set `local.foundPlayer` false)
  (set `local.foundEnemy` false)
  (for _array_element (`PrimitiveComponent.GetOverlappingActors` (`self.RoomBoxVolume`) null)
    (bind _asbp_enemy (cast `/Game/Blueprint/AI/Enemies/BP_Enemy` _array_element)
      (:`then`
        (if (not (`/Game/Blueprint/AI/Enemies/BP_Enemy.isDead` _asbp_enemy))
          (set `local.foundEnemy` true)))
      (:`CastFailed`
        (cast `/Game/Blueprint/Character/BP_Oubliette_Character` _array_element)
        (set `local.foundPlayer` true))))
  (if _foundplayer
    (set `/Game/Blueprint/BP_GameModeOubliette.isInCombat` (and (`local.foundEnemy`) _foundplayer) (cast `/Game/Blueprint/BP_GameModeOubliette` (`GameplayStatics.GetGameMode`) :!pure true))))

(fn `UserConstructionScript`)