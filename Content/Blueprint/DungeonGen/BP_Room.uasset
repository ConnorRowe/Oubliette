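; BP_Room is a dungeon room actor that spawns an enemy and tracks whether the player is in combat there.
; On BeginPlay it spawns a slime at an offset from itself, usually fire and occasionally giant, then starts a looping timer.
; The timer polls the Box's overlapping actors and, when the player is inside, sets the game mode's IsInCombat by whether a living enemy is present.
; A helper writes an iteration number to a text render.
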(event `self.ReceiveBeginPlay`
  (`|SpawnActorFromClass` (castclass `/Game/Blueprint/AI/Enemies/BP_Enemy` (select `bool` (> (`KismetMathLibrary.RandomIntegerInRange` 0 5) 0) :`false` "/Game/Blueprint/AI/Enemies/BP_Enemy_Slime_Giant.BP_Enemy_Slime_Giant_C" :`true` "/Game/Blueprint/AI/Enemies/BP_Enemy_Slime_Fire.BP_Enemy_Slime_Fire_C" :!type "Actor Class Reference") :!pure true) (`KismetMathLibrary.MakeTransform` (+ (`self.K2_GetActorLocation`) (400.0 0.0 0.0))) "AdjustIfPossibleButAlwaysSpawn" "OverrideRootScale" null (struct) null)
  (`KismetSystemLibrary.K2_SetTimer` null "CheckForCombat" 0.5 true))

(fn `CheckForCombat`
  (locals (foundEnemy :type Boolean) (foundPlayer :type Boolean))
  (bind _foundplayer (`local.foundPlayer`))
  (set `local.foundPlayer` false)
  (set `local.foundEnemy` false)
  (for _array_element (`PrimitiveComponent.GetOverlappingActors` (`self.Box`) null)
    (bind _asbp_enemy (cast `/Game/Blueprint/AI/Enemies/BP_Enemy` _array_element)
      (:`then`
        (if (not (`/Game/Blueprint/AI/Enemies/BP_Enemy.isDead` _asbp_enemy))
          (set `local.foundEnemy` true)))
      (:`CastFailed`
        (cast `/Game/Blueprint/Character/BP_Oubliette_Character` _array_element)
        (set `local.foundPlayer` true))))
  (if _foundplayer
    (set `/Game/Blueprint/Oubliette_GameMOde.isInCombat` (and (`local.foundEnemy`) _foundplayer) (cast `/Game/Blueprint/Oubliette_GameMOde` (`GameplayStatics.GetGameMode`) :!pure true))))

(fn `UpdateRoomTestText`
  (params (Iteration :type Integer))
  (`TextRenderComponent.K2_SetText` (`self.TextRender`) (`KismetTextLibrary.Conv_IntToText` Iteration)))

(fn `UserConstructionScript`)