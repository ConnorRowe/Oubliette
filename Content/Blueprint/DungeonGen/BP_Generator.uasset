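; Dungeon generator actor that builds a random chain of BP_Room actors on BeginPlay.
; GenerateRoom records candidate positions, offsetting each from a stored one in a random cardinal direction.
; TryPlaceRoom spawns a room unless an upward line trace finds the spot occupied; failures decrement the loop index, with iterations capped.
; Each success places a door on the previous room using a direction rolled separately from the offset.
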(event `self.ReceiveBeginPlay`
  (bind _lastroom (`self.LastRoom`))
  (for _index (range (+ (`self.DungeonSize`) 1))
    (bind (_roomlocation _gendirection) (`self.GenerateRoom` _index))
    (bind (_return_bool _return_room) (`self.TryPlaceRoom` _roomlocation))
    (if _return_bool
      (`/Engine/EditorBlueprintResources/StandardMacros.IsValid` _lastroom
        (:`Is Valid`
          (`/Game/Blueprint/DungeonGen/BP_Room.PlaceDoor` _lastroom _gendirection))
        (:`Is Not Valid`
          _))
      (bind _output_get (set `self.LastRoom` _return_room))
      (`/Game/Blueprint/DungeonGen/BP_Room.UpdateRoomTestText` _output_get _index)
      (else
        (`/Engine/EditorBlueprintResources/StandardMacros.DecrementInt` _index
          (:`  `
            _))))
    (`/Engine/EditorBlueprintResources/StandardMacros.IncrementInt` (`self.RoomIteration`)
      (:`  `
        (if (>= (`self.RoomIteration`) 100)
          (break))))))

(fn `GenerateRoom`
  (params (Iteration :type Integer))
  (returns (RoomLocation :type "Vector Structure") (GenDirection :type Integer))
  (locals (NewLocation :type "Vector Structure"))
  (bind _returnvalue (`KismetMathLibrary.RandomIntegerInRange` 0 3))
  (bind _newlocation (`local.NewLocation`))
  (if (== Iteration 0)
    (set `local.NewLocation` (`self.K2_GetActorLocation`))
    (else
      (set `local.NewLocation` (+ (`|GetArrayItem` (`self.RoomPositions`) (- Iteration 1)) (select `int` _returnvalue :`0` (2000.0 0.0 0.0) :`1` (-2000.0 0.0 0.0) :`2` (0.0 2000.0 0.0) :`3` (0.0 -2000.0 0.0) :!type "Vector Structure")))))
  (`KismetArrayLibrary.Array_Add` (`self.RoomPositions`) _newlocation)
  (return _newlocation _returnvalue))

(fn `TryPlaceRoom`
  (params (RoomLocation :type "Vector Structure"))
  (returns (`Return Bool` :type Boolean) (`Return Room` :type "/Game/Blueprint/DungeonGen/BP_Room Object Reference"))
  (locals (NotOverlapping :type Boolean :default true) (RoomPosition :type "Vector Structure") (RoomSize :type "Vector Structure"))
  (bind (_outhit _returnvalue) (`KismetSystemLibrary.LineTraceSingleForObjects` :`Start` RoomLocation :`End` (+ RoomLocation (0.0 0.0 200.0)) :`ObjectTypes` (`|MakeArray` "ObjectTypeQuery4" "ObjectTypeQuery1" "ObjectTypeQuery2" :!type "EObjectTypeQuery Enum") :`DrawDebugType` "Persistent"))
  (if _returnvalue
    (return false null)
    (else
      (bind _returnvalue_2 (`|SpawnActorFromClass` "/Game/Blueprint/DungeonGen/BP_Room.BP_Room_C" (`KismetMathLibrary.Conv_VectorToTransform` RoomLocation) "Undefined" "OverrideRootScale" null null))
      (return true _returnvalue_2))))

(fn `UserConstructionScript`)