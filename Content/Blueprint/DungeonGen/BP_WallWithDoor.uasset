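; BP_WallWithDoor is a dungeon wall with a two-part door that opens for the player and locks during combat.
; A fast looping timer checks the game mode's combat state and Box overlaps with Oubliette_Character, then opens, closes or locks the door.
; TL_Door slides both parts, reversing after a short delay to close.
; At BeginPlay the actor destroys itself unless its yaw is zero or its rotation is near 90 degrees yaw.
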(event `OpenDoor`
  (bind (_direction _door1 _door2) (`Timeline|TL_Door` :!label _label)
    (:`Update`
      (switch `ETimelineDirection` _direction
        (:`Forward`
          (set `self.isOpen` true))
        (:`Backward`
          _))
      (`SceneComponent.K2_SetRelativeLocation` (`self.Door1`) _door1 false true)
      (`SceneComponent.K2_SetRelativeLocation` (`self.Door2`) _door2 false true))
    (:`Finished`
      (switch `ETimelineDirection` _direction
        (:`Backward`
          (set `self.isOpen` false))))))

(event `CloseDoor`
  (`KismetSystemLibrary.Delay` 0.3)
  (goto _label :!via `Reverse`))

(event `self.ReceiveBeginPlay`
  (bind _returnvalue (`self.K2_GetActorRotation`))
  (`KismetSystemLibrary.K2_SetTimer` null "CheckForPlayer" 0.01 true)
  (if (and (!= _returnvalue (struct :`Yaw` 90.0) :`ErrorTolerance` 20.0) (!= (.yaw _returnvalue) 0.0))
    (`self.K2_DestroyActor`)))

(fn `CheckForPlayer`
  (if (`/Game/Blueprint/Oubliette_GameMOde.isInCombat` (cast `/Game/Blueprint/Oubliette_GameMOde` (`GameplayStatics.GetGameMode`) :!pure true))
    (`self.Lock`)
    (else
      (`self.Unlock`)
      (if (> (`KismetArrayLibrary.Array_Length` (`PrimitiveComponent.GetOverlappingActors` (`self.Box`) "/Game/Blueprint/Character/Oubliette_Character.Oubliette_Character_C")) 0)
        (if (`self.canOpen`)
          (`self.OpenDoor`)
          (else
            (`self.CloseDoor` :!label _label)))
        (else
          (goto _label))))))

(fn `Lock`
  (`self.CloseDoor`)
  (set `self.canOpen` false))

(fn `Unlock`
  (set `self.canOpen` true))

(fn `UserConstructionScript`)