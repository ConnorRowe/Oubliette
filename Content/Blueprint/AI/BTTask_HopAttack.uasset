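; Behavior tree task that starts a hop attack on an AI-controlled BP_Enemy.
; On execute it gets the enemy pawn through a cached BP_EnemyAIController reference, filling that cache from the task owner when unset.
; It only raises the enemy's IsJumping and IsAttacking flags and reports success immediately, without waiting for the attack.
; A failed cast never calls FinishExecute.
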(event `self.ReceiveExecute`
  (params (OwnerActor :type "Actor Object Reference"))
  (if (not (!= (`self.AI_CON_REF`) null))
    (bind _asbp_enemy_aicontroller (cast `/Game/Blueprint/BP_EnemyAIController` OwnerActor))
    (set `self.AI_CON_REF` _asbp_enemy_aicontroller))
  (bind _asbp_enemy (cast `/Game/Blueprint/AI/Enemies/BP_Enemy` (`Controller.K2_GetPawn` (`self.AI_CON_REF`))))
  (set `/Game/Blueprint/AI/Enemies/BP_Enemy.isJumping` true _asbp_enemy)
  (set `/Game/Blueprint/AI/Enemies/BP_Enemy.isAttacking` true _asbp_enemy)
  (`self.FinishExecute` true))