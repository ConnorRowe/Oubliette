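; Giant slime enemy Blueprint that splits into smaller slimes when it dies.
; It overrides the dying event, runs the parent behavior, then spawns three or four regular slimes, with a random boolean setting the loop's start index.
; Each spawns at a random point in a wide, nearly flat box around the giant's location, adjusting for collisions but always spawning.
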(event `/Game/Blueprint/AI/Enemies/BP_Enemy.DyingActions`
  (`parent.DyingActions`)
  (for _ (range (`KismetMathLibrary.Conv_BoolToInt` (`KismetMathLibrary.RandomBool`)) 4)
    (`|SpawnActorFromClass` "/Game/Blueprint/AI/Enemies/BP_Enemy_Slime.BP_Enemy_Slime_C" (`KismetMathLibrary.MakeTransform` (`KismetMathLibrary.RandomPointInBoundingBox` (`self.K2_GetActorLocation`) (600.0 600.0 1.0))) "AdjustIfPossibleButAlwaysSpawn" "OverrideRootScale" null (struct) null)))

(fn `UserConstructionScript`
  (`parent.UserConstructionScript`))