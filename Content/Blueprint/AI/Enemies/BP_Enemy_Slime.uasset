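; Slime enemy character that moves by leaping, with a colour-tinted body and slime particle effects.
; LeapForwards jumps with a sound, then after a short delay adds a forward impulse that is stronger while attacking.
; Landing clears the attack state, sets a landing flag, plays a splat and pulses the Niagara burst alongside a particle event.
; The construction script feeds the base and dark colours into the mesh materials and the base colour into the Niagara system.
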(event `LeapForwards`
  (`self.Jump`)
  (`GameplayStatics.PlaySoundAtLocation` "/Game/Sound/Slime_Jump_Cue.Slime_Jump_Cue" (`self.K2_GetActorLocation`) (struct) 1.0 1.0 0.0 null null null)
  (`KismetSystemLibrary.Delay` 0.2)
  (`CharacterMovementComponent.AddImpulse` (`self.CharacterMovement`) (* (`KismetMathLibrary.GetForwardVector` (`self.K2_GetActorRotation`)) (select `bool` (`self.isAttacking`) :`false` 160.0 :`true` 500.0 :!type "Float (single-precision)")) true))

(event `self.OnLanded`
  (params (Hit :type "HitResult Structure (by ref)"))
  (bind _returnvalue (`self.K2_GetActorLocation`))
  (bind _ns_slime (`self.NS_Slime`))
  (`ParticleSystemComponent.GenerateParticleEvent` (`self.ParticleSystem`) "BurstEvent" 0.0 _returnvalue (0.0 0.0 0.0) (0.0 0.0 0.0))
  (set `self.isAttacking` false)
  (`GameplayStatics.PlaySoundAtLocation` "/Game/Sound/Splat_Cue.Splat_Cue" _returnvalue (struct) 1.0 1.0 0.0 null null null)
  (set `self.isLanding` true)
  (`NiagaraComponent.SetNiagaraVariableBool` _ns_slime "User.SpawnBurst" true)
  (`KismetSystemLibrary.Delay` 0.1)
  (`NiagaraComponent.SetNiagaraVariableBool` _ns_slime "User.SpawnBurst" false))

(fn `UserConstructionScript`
  (bind _mesh (`self.Mesh`))
  (`parent.UserConstructionScript`)
  (`MeshComponent.SetVectorParameterValueOnMaterials` _mesh "Colour" (`KismetMathLibrary.Conv_LinearColorToVector` (`self.BaseColour`)))
  (`MeshComponent.SetVectorParameterValueOnMaterials` _mesh "ColourDark" (`KismetMathLibrary.Conv_LinearColorToVector` (`self.DarkColour`)))
  (`NiagaraComponent.SetNiagaraVariableLinearColor` (`self.NS_Slime`) "User.ParticleColour" (`self.BaseColour`)))