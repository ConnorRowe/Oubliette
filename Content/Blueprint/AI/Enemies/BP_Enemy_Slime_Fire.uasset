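; Fire slime enemy Blueprint that supplies its ranged attack.
; The ShootProjectile event spawns a BP_EnemyProjectile_FireSlimeball slightly above the actor's location.
; BeginPlay, overlap and Tick are unused stubs, and the construction script only calls the parent.
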(event `/Game/Blueprint/AI/Enemies/BP_Enemy.ShootProjectile`
  (`|SpawnActorFromClass` "/Game/Blueprint/AI/Enemies/Projectiles/BP_EnemyProjectile_FireSlimeball.BP_EnemyProjectile_FireSlimeball_C" (`KismetMathLibrary.MakeTransform` (+ (`self.K2_GetActorLocation`) (0.0 0.0 100.0))) "Undefined" "OverrideRootScale" null 1.0 null))

(fn `UserConstructionScript`
  (`parent.UserConstructionScript`))