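; Melee walking enemy that can leap forward and strike the player character, extending a parent class.
; LeapForwards jumps, adds a delayed forward velocity impulse, and holds CanLeap false for a cooldown.
; DealMeleeDamage box-traces ahead of the static mesh, applying arcane damage and a hit sound to the first hit if it is BP_Oubliette_Character.
; DyingActions turns on physics for both meshes and makes the static mesh block all channels.
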(event `self.ReceiveBeginPlay`
  (`parent.ReceiveBeginPlay`))

(event `self.ReceiveActorBeginOverlap`
  (params (OtherActor :type "Actor Object Reference"))
  (`parent.ReceiveActorBeginOverlap` OtherActor))

(event `self.ReceiveTick`
  (params (DeltaSeconds :type "Float (single-precision)"))
  (`parent.ReceiveTick` DeltaSeconds))

(event `Leap Forwards`
  (set `self.canLeap` false)
  (`self.Jump`)
  (`KismetSystemLibrary.Delay` 0.2)
  (`CharacterMovementComponent.AddImpulse` (`self.CharacterMovement`) (* (`KismetMathLibrary.GetForwardVector` (`self.K2_GetActorRotation`)) 800.0) true)
  (`KismetSystemLibrary.Delay` 5.0)
  (set `self.canLeap` true))

(event `self.DyingActions`
  (`PrimitiveComponent.SetSimulatePhysics` (`self.Mesh`) true)
  (`PrimitiveComponent.SetSimulatePhysics` (`self.StaticMesh`) true)
  (`PrimitiveComponent.SetCollisionResponseToAllChannels` (`self.StaticMesh`) "ECR_Block"))

(fn `DealMeleeDamage`
  (bind _staticmesh (`self.StaticMesh`))
  (bind _returnvalue (`SceneComponent.K2_GetComponentLocation` _staticmesh))
  (bind _outhits (`KismetSystemLibrary.BoxTraceMulti` :`Start` _returnvalue :`End` (+ _returnvalue (* (`SceneComponent.GetForwardVector` _staticmesh) 20.0)) :`HalfSize` (25.0 80.0 50.0) :`Orientation` (`SceneComponent.K2_GetComponentRotation` _staticmesh) :`TraceChannel` "TraceTypeQuery2" :`bTraceComplex` true :`DrawTime` 2.0))
  (for _array_element _outhits
    (bind _asbp_oubliette_character (cast `/Game/Blueprint/Character/BP_Oubliette_Character` (`.HitActor` (`GameplayStatics.BreakHitResult` _array_element))))
    (`GameplayStatics.ApplyDamage` _asbp_oubliette_character 1.0 null self "/Script/Oubliette.MyDamageType_Arcane")
    (`GameplayStatics.PlaySoundAtLocation` "/Game/Sound/PlayerHt_Cue.PlayerHt_Cue" (`.Location` (`GameplayStatics.BreakHitResult` _array_element)) (struct) 1.0 1.0 0.0 null null null)
    (break)))

(fn `UserConstructionScript`
  (`parent.UserConstructionScript`))