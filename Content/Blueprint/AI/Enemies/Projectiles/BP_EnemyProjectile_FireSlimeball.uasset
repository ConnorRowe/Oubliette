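; Fire slimeball variant of an enemy projectile, with its core behavior left to the parent class.
; The construction script runs the parent's setup, then tints the projectile mesh orange through the material "Colour" parameter.
; The Die event simply destroys the actor, while BeginPlay, overlap and Tick are unused disabled stubs.
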(event `self.Die`
  (`self.K2_DestroyActor`))

(fn `UserConstructionScript`
  (`parent.UserConstructionScript`)
  (`MeshComponent.SetVectorParameterValueOnMaterials` (`self.ProjMesh`) "Colour" (`KismetMathLibrary.Conv_LinearColorToVector` (struct :`R` 0.67451 :`G` 0.313726 :`B` 0.082353 :`A` 1.0))))