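; Base-style enemy projectile that damages the Oubliette player character on overlap, then destroys itself.
; The construction script applies homing and speed variables to ProjectileMovement, using speed as the homing acceleration.
; On BeginPlay it targets the game instance's stored character root for homing and starts a lifetime timer calling Die, which is empty here.
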(event `self.ReceiveBeginPlay`
  (`KismetSystemLibrary.K2_SetTimer` null "Die" (`self.Lifetime`))
  (if true
    (set `ProjectileMovementComponent.HomingTargetComponent` (`Actor.RootComponent` (`GameInstanceOubliette.charRef` (cast `/Game/Blueprint/BP_OublietteGameInstance` (`GameplayStatics.GetGameInstance`) :!pure true))) (`self.ProjectileMovement`))))

(event `self.ReceiveActorBeginOverlap`
  (params (OtherActor :type "Actor Object Reference"))
  (bind _asbp_oubliette_character (cast `/Game/Blueprint/Character/BP_Oubliette_Character` OtherActor))
  (`GameplayStatics.ApplyDamage` _asbp_oubliette_character (`self.Damage`) null (`self.GetInstigator`) (`self.DamageType`))
  (`self.K2_DestroyActor`))

(fn `Die`)

(fn `UserConstructionScript`
  (bind _projectilemovement (`self.ProjectileMovement`))
  (bind _projectilespeed (`self.ProjectileSpeed`))
  (set `ProjectileMovementComponent.bIsHomingProjectile` (`self.isHoming`) _projectilemovement)
  (set `ProjectileMovementComponent.MaxSpeed` _projectilespeed _projectilemovement)
  (if true
    (set `ProjectileMovementComponent.HomingAccelerationMagnitude` _projectilespeed _projectilemovement)))