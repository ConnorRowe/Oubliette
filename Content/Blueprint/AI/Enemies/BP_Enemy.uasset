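; Base enemy character with stats-driven health, a floating health bar, damage numbers and a death sequence.
; Spell projectile hits become AnyDamage, which filters causers by allowed classes, then lowers health and spawns damage text.
; At zero health it marks itself dying, ignores key collision channels and calls the empty DyingActions hook.
; A looping timer toggles the health bar by target range, while Tick eases yaw toward TargetLocation.
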(event `DyingActions`)

(event `self.ReceiveAnyDamage`
  (params (Damage :type "Float (single-precision)") (DamageType :type "DamageType Object Reference") (InstigatedBy :type "Controller Object Reference") (DamageCauser :type "Actor Object Reference"))
  (bind _capsulecomponent (`self.CapsuleComponent`))
  (bind _newparam (`self.CanBeDamagedByClass` DamageCauser))
  (if (and _newparam (not (or (`self.isDying`) (`self.isDead`))))
    (set `self.HealthCurrent` (- (`self.HealthCurrent`) Damage))
    (`self.SpawnDamageWidget` (`KismetMathLibrary.FTrunc` (* Damage 10.0)))
    (if (< (`self.HealthCurrent`) (`self.HealthMax`))
      (`SceneComponent.SetVisibility` (`self.HealthBarWidget`) true false)
      (if (<= (`self.HealthCurrent`) 0.0)
        (`/Engine/EditorBlueprintResources/StandardMacros.DoOnce` false
          (:`Completed`
            (set `self.isDying` true)
            (`SceneComponent.SetVisibility` (`self.HealthBarWidget`) false false)
            (`ActorComponent.Deactivate` (`self.ParticleSystem`))
            (`PrimitiveComponent.SetCollisionResponseToChannel` _capsulecomponent "ECC_Pawn" "ECR_Ignore")
            (`PrimitiveComponent.SetCollisionResponseToChannel` (`self.BoxCollision`) "ECC_Pawn" "ECR_Ignore")
            (`PrimitiveComponent.SetCollisionResponseToChannel` _capsulecomponent "ECC_GameTraceChannel1" "ECR_Ignore")
            (`PrimitiveComponent.SetCollisionResponseToChannel` (`self.BoxCollision`) "ECC_GameTraceChannel1" "ECR_Ignore")
            (`PrimitiveComponent.SetCollisionResponseToChannel` (`self.BoxCollision`) "ECC_Camera" "ECR_Ignore")
            (`PrimitiveComponent.SetCollisionResponseToChannel` _capsulecomponent "ECC_Camera" "ECR_Ignore")
            (`self.DyingActions`)))))))

(event `self.ReceiveBeginPlay`
  (bind (_hp _perceptiondistance _name) (break `/Game/Blueprint/AI/Enemies/EnemyStats` (`self.BaseStats`)))
  (set `self.HealthMax` _hp)
  (set `self.PerceptionDistance` _perceptiondistance)
  (set `self.EnemyName` _name)
  (set `self.HealthCurrent` (`self.HealthMax`))
  (bind _asui_enemy_health_bar (cast `/Game/Blueprint/UI/UI_Enemy_HealthBar` (`WidgetComponent.GetUserWidgetObject` (`self.HealthBarWidget`))))
  (set `/Game/Blueprint/UI/UI_Enemy_HealthBar.EnemyNameT` (`KismetTextLibrary.Conv_NameToText` (`self.EnemyName`)) _asui_enemy_health_bar)
  (set `/Game/Blueprint/UI/UI_Enemy_HealthBar.EnemyRef` self _asui_enemy_health_bar)
  (`KismetSystemLibrary.K2_SetTimerDelegate` (delegate `HideHealthBarCheck`) 5.0 true))

(event `HideHealthBarCheck`
  (bind _healthbarwidget (`self.HealthBarWidget`))
  (bind _inrange (`self.CheckTargetRange`))
  (if (not _inrange)
    (`SceneComponent.SetVisibility` _healthbarwidget false false)
    (elif (and (< (`self.HealthCurrent`) (`self.HealthMax`)) (> (`self.HealthCurrent`) 0.0))
      (`SceneComponent.SetVisibility` _healthbarwidget true false))))

(event `self.ReceiveTick`
  (params (DeltaSeconds :type "Float (single-precision)"))
  (`self.LookToActor`)
  (set `self.HealthPercentage` (/ (`self.HealthCurrent`) (`self.HealthMax`))))

(event `UpdateTurnToFace`
  (params (`shouldTurn?` :type Boolean) (TargetLocation :type "Vector Structure"))
  (set `self.shouldTurntoFace` `shouldTurn?`)
  (set `self.TargetLocation` TargetLocation))

(event `self.ReceiveHit`
  (params (MyComp :type "PrimitiveComponent Object Reference") (Other :type "Actor Object Reference") (OtherComp :type "PrimitiveComponent Object Reference") (bSelfMoved :type Boolean) (HitLocation :type "Vector Structure") (HitNormal :type "Vector Structure") (NormalImpulse :type "Vector Structure") (Hit :type "HitResult Structure (by ref)"))
  (bind _asbp_spell_projectile (cast `/Game/Blueprint/Spells/Projectile/BP_Spell_Projectile` Other))
  (`GameplayStatics.ApplyDamage` self (`OublietteSpell.spellDamage` _asbp_spell_projectile) (`self.GetInstigatorController` _asbp_spell_projectile) (`self.GetInstigator` _asbp_spell_projectile) (`OublietteSpell.damageType` _asbp_spell_projectile)))

(fn `CanBeDamagedByClass`
  (params (Object :type "Object Object Reference"))
  (returns (NewParam :type Boolean))
  (locals (`CanBeDamaged?` :type Boolean :default false))
  (bind _returnvalue (`GameplayStatics.GetObjectClass` Object))
  (for _array_element (`self.DamageAbleClasses`)
    (if (== _array_element _returnvalue)
      (set `local.CanBeDamaged?` true)
      (break)
      (elif (`KismetMathLibrary.ClassIsChildOf` _returnvalue _array_element)
        (set `local.CanBeDamaged?` true)
        (break))))
  (return (`local.CanBeDamaged?`)))

(fn `CheckTargetRange`
  (returns (InRange :type Boolean))
  (bind _target (`self.Target`))
  (`/Engine/EditorBlueprintResources/StandardMacros.IsValid` _target
    (:`Is Valid`
      (return (<= (`KismetMathLibrary.VSize` (- (`self.K2_GetActorLocation` _target) (`self.K2_GetActorLocation`))) (`self.PerceptionDistance`))))
    (:`Is Not Valid`
      (return false))))

(fn `LookToActor`
  (bind _returnvalue (`self.K2_GetActorLocation`))
  (bind (_returnvalue_roll _returnvalue_pitch _returnvalue_yaw) (`KismetMathLibrary.BreakRotator` (`KismetMathLibrary.FindLookAtRotation` _returnvalue (`self.TargetLocation`))))
  (`self.isDyingOrDead`
    (:`False`
      (if (!= _returnvalue (`self.TargetLocation`))
        (if (`NavMovementComponent.IsMovingOnGround` (`self.CharacterMovement`))
          (`self.K2_SetActorRotation` (`KismetMathLibrary.RLerp` (`self.K2_GetActorRotation`) (`KismetMathLibrary.MakeRotator` 0.0 0.0 _returnvalue_yaw) (* (`GameplayStatics.GetWorldDeltaSeconds`) 1.5) true)))))))

(fn `ShootProjectile`)

(fn `SpawnDamageWidget`
  (params (Damage :type Integer) (isCrit :type Boolean))
  (bind _returnvalue (`AddComponent|NODE_AddWidgetComponent-0` :`RelativeTransform` (`KismetMathLibrary.MakeTransform` (`KismetMathLibrary.RandomPointInBoundingBox` (-10.0 -10.0 0.0) (10.0 10.0 10.0)))))
  (bind _asdamage_text (cast `/Game/Blueprint/UI/DamageText` (`WidgetComponent.GetUserWidgetObject` _returnvalue)))
  (`/Game/Blueprint/UI/DamageText.init` _asdamage_text Damage isCrit _returnvalue))

(fn `UserConstructionScript`)