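; Behavior tree task that moves an enemy's pawn to the actor stored in the TargetToFollow blackboard value.
; On execute it reuses a cached BP_EnemyAIController reference, or casts the owner to one and stores it on first use.
; It then runs AI MoveTo with a small acceptance radius and stop-on-overlap, finishing successfully on arrival.
; A failed move or cast never calls Finish Execute.
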(event `self.ReceiveExecute`
  (params (OwnerActor :type "Actor Object Reference"))
  (if (not (!= (`self.AI_CON_REF`) null))
    (bind _asbp_enemy_aicontroller (cast `/Game/Blueprint/BP_EnemyAIController` OwnerActor))
    (set `self.AI_CON_REF` _asbp_enemy_aicontroller))
  (`|AIMoveTo` (`Controller.K2_GetPawn` (`self.AI_CON_REF`)) (0.0 0.0 0.0) (`BTFunctionLibrary.GetBlackboardValueAsActor` (`self.TargetToFollow`)) 50.0 true
    (:`OnSuccess`
      (`self.FinishExecute` true))))