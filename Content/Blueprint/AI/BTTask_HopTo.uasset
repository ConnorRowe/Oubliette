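; Behavior tree task that makes an AI-controlled BP_Enemy hop forward.
; It caches the owning BP_EnemyAIController on first execution and gets the enemy pawn from it.
; The enemy jumps, then after a short delay receives a velocity-change impulse along its facing direction before the task finishes successfully.
; Failed casts end the flow without calling FinishExecute.
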(event `self.ReceiveExecute`
  (params (OwnerActor :type "Actor Object Reference"))
  (if (not (!= (`self.AI_CON_REF`) null))
    (bind _asbp_enemy_aicontroller (cast `/Game/Blueprint/BP_EnemyAIController` OwnerActor))
    (set `self.AI_CON_REF` _asbp_enemy_aicontroller))
  (bind _asbp_enemy (cast `/Game/Blueprint/BP_Enemy` (`Controller.K2_GetPawn` (`self.AI_CON_REF`))))
  (`Character.Jump` _asbp_enemy)
  (`KismetSystemLibrary.Delay` 0.2)
  (`CharacterMovementComponent.AddImpulse` (`Character.CharacterMovement` _asbp_enemy) (* (`KismetMathLibrary.GetForwardVector` (`Actor.K2_GetActorRotation` _asbp_enemy)) 125.0) true)
  (`self.FinishExecute` true))