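; Behavior tree decorator that passes when the AI-controlled enemy pawn is facing a target actor.
; It casts the owner to BP_EnemyAIController and reads the target from the TargetToTurnTo blackboard key.
; The check compares the look-at yaw toward the target with the pawn's current yaw within a Tolerance, ignoring pitch and roll.
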(fn `PerformConditionCheck`
  (params (OwnerActor :type "Actor Object Reference"))
  (returns (ReturnValue :type Boolean))
  (bind _returnvalue (`Controller.K2_GetPawn` (`self.AI_CON_REF`)))
  (bind (_returnvalue_roll _returnvalue_pitch _returnvalue_yaw) (`KismetMathLibrary.BreakRotator` (`Actor.K2_GetActorRotation` _returnvalue)))
  (bind (_returnvalue_roll_2 _returnvalue_pitch_2 _returnvalue_yaw_2) (`KismetMathLibrary.BreakRotator` (`KismetMathLibrary.FindLookAtRotation` (`Actor.K2_GetActorLocation` _returnvalue) (`Actor.K2_GetActorLocation` (`BTFunctionLibrary.GetBlackboardValueAsActor` (`self.TargetToTurnTo`))))))
  (bind _asbp_enemy_aicontroller (cast `/Game/Blueprint/BP_EnemyAIController` OwnerActor))
  (set `self.AI_CON_REF` _asbp_enemy_aicontroller)
  (return (`KismetMathLibrary.NearlyEqual_FloatFloat` _returnvalue_yaw_2 _returnvalue_yaw (`self.Tolerance`))))