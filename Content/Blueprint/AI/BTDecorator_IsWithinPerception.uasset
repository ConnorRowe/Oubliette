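; Behavior tree decorator that checks whether an enemy's TargetToFollow actor is within its perception range.
; It casts the owner to BP_EnemyAIController and reads the target actor from the blackboard.
; The condition passes when the straight-line distance from the controlled pawn to the target is at most that BP_Enemy's PerceptionDistance.
; The test is purely distance-based, with no line-of-sight or AI Perception query.
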(fn `PerformConditionCheck`
  (params (OwnerActor :type "Actor Object Reference"))
  (returns (ReturnValue :type Boolean))
  (bind _asbp_enemy_aicontroller (cast `/Game/Blueprint/BP_EnemyAIController` OwnerActor))
  (set `self.AI_CON_REF` _asbp_enemy_aicontroller)
  (return (<= (`KismetMathLibrary.VSize` (- (`Actor.K2_GetActorLocation` (`BTFunctionLibrary.GetBlackboardValueAsActor` (`self.TargetToFollow`))) (`Actor.K2_GetActorLocation` (`Controller.K2_GetPawn` (`self.AI_CON_REF`))))) (`/Game/Blueprint/AI/Enemies/BP_Enemy.PerceptionDistance` (cast `/Game/Blueprint/AI/Enemies/BP_Enemy` (`Controller.K2_GetPawn` _asbp_enemy_aicontroller) :!pure true)))))