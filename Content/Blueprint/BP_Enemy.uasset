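; BP_Enemy is an enemy actor that takes filtered damage and can turn to face a target.
; AnyDamage lowers current health only when the causer's class matches or derives from an entry in DamageAbleClasses; no death logic follows.
; UpdateTurnToFace sets the target and flag that Tick uses to apply look-at yaw, effectively snapping.
; Landing fires a particle burst event, while the AI perception handler is empty.
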(event `self.AIPerception.OnTargetPerceptionUpdated`
  (params (Actor :type "Actor Object Reference") (Stimulus :type "AIStimulus Structure")))

(event `self.ReceiveAnyDamage`
  (params (Damage :type "Float (single-precision)") (DamageType :type "DamageType Object Reference") (InstigatedBy :type "Controller Object Reference") (DamageCauser :type "Actor Object Reference"))
  (bind _newparam (`self.CanBeDamagedByClass` DamageCauser))
  (if _newparam
    (set `self.HealthCurrent` (- (`self.HealthCurrent`) Damage))))

(event `self.ReceiveBeginPlay`)

(event `UpdateTurnToFace`
  (params (`shouldTurn?` :type Boolean) (Target :type "Actor Object Reference"))
  (set `self.shouldTurntoFace` `shouldTurn?`)
  (set `self.Target` Target))

(event `self.ReceiveTick`
  (params (DeltaSeconds :type "Float (single-precision)"))
  (`self.LookToActor`))

(event `self.ParticleSystem.OnParticleBurst`
  (params (EventName :type Name) (EmitterTime :type "Float (single-precision)") (ParticleCount :type Integer)))

(event `self.OnLanded`
  (params (Hit :type "HitResult Structure (by ref)"))
  (`ParticleSystemComponent.GenerateParticleEvent` (`self.ParticleSystem`) "BurstEvent" 0.0 (`self.K2_GetActorLocation`) (0.0 0.0 0.0) (0.0 0.0 0.0)))

(fn `CanBeDamagedByClass`
  (params (Object :type "Object Object Reference"))
  (returns (NewParam :type Boolean))
  (locals (`CanBeDamaged?` :type Boolean :default false))
  (bind _returnvalue (`GameplayStatics.GetObjectClass` Object))
  (for _array_element (`self.DamageAbleClasses`)
    (if (== _array_element _returnvalue)
      (set `local.CanBeDamaged?` true)
      (break)
      (elif (`KismetMathLibrary.ClassIsChildOf` _returnvalue _array_element)
        (set `local.CanBeDamaged?` true)
        (break))))
  (return (`local.CanBeDamaged?`)))

(fn `LookToActor`
  (bind _returnvalue (`KismetMathLibrary.FindLookAtRotation` (`self.K2_GetActorLocation`) (`self.K2_GetActorLocation` (`self.Target`))))
  (bind (_returnvalue_roll _returnvalue_pitch _returnvalue_yaw) (`KismetMathLibrary.BreakRotator` (`KismetMathLibrary.ComposeRotators` _returnvalue (* (`KismetMathLibrary.NormalizedDeltaRotator` _returnvalue (`self.K2_GetActorRotation`)) (* (`GameplayStatics.GetWorldDeltaSeconds`) 1e-05)))))
  (if (`self.shouldTurntoFace`)
    (`/Engine/EditorBlueprintResources/StandardMacros.IsValid` (`self.Target`)
      (:`Is Valid`
        (`self.K2_SetActorRotation` (`KismetMathLibrary.MakeRotator` 0.0 0.0 _returnvalue_yaw))))))

(fn `UserConstructionScript`)