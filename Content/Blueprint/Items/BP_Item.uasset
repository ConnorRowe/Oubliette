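; BP_Item is a world item pickup that hands itself to the player character through PickupItem on interact.
; Init stores the item data, tints the beam and box by rarity, and fills the tooltip and slot widgets; selection is forwarded to the tooltip.
; Looping timers, used instead of Tick, keep the beam on the box, show both widgets near the player, and yaw them toward the player.
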(event `/Game/Blueprint/BPI_Interactable.Interact`
  (`/Game/Blueprint/Character/BP_Oubliette_Character.PickupItem` (`self.CharRef`) self))

(event `/Game/Blueprint/BPI_Selectable.SelectObject`
  (params (isSelected :type Boolean))
  (`/Game/Blueprint/UI/UI_ItemTooltip.SetSelected` (cast `/Game/Blueprint/UI/UI_ItemTooltip` (`WidgetComponent.GetUserWidgetObject` (`self.ItemTooltipWidget`)) :!pure true) isSelected))

(event `self.ReceiveBeginPlay`
  (set `self.CharRef` (cast `/Game/Blueprint/Character/BP_Oubliette_Character` (`GameInstanceOubliette.charRef` (cast `GameInstanceOubliette` (`GameplayStatics.GetGameInstance`) :!pure true)) :!pure true))
  (`KismetSystemLibrary.K2_SetTimer` null "BeamFollowItem" 0.02 true)
  (`KismetSystemLibrary.K2_SetTimer` null "CheckPlayerRange" 0.1 true))

(event `Init`
  (params (Item :type "ItemStruct Structure"))
  (set `self.ItemData` Item)
  (`MeshComponent.SetVectorParameterValueOnMaterials` (`self.Beam`) "Colour" (`KismetMathLibrary.Conv_LinearColorToVector` (`BlueprintMapLibrary.Map_Find` (`self.RarityColours`) (`.Rarity` (break `ItemStruct` (`self.ItemData`))))))
  (`MeshComponent.SetVectorParameterValueOnMaterials` (`self.Box`) "Colour" (`KismetMathLibrary.Conv_LinearColorToVector` (`BlueprintMapLibrary.Map_Find` (`self.RarityColours`) (`.Rarity` (break `ItemStruct` (`self.ItemData`))))))
  (bind _asui_item_tooltip (cast `/Game/Blueprint/UI/UI_ItemTooltip` (`WidgetComponent.GetUserWidgetObject` (`self.ItemTooltipWidget`))))
  (`/Game/Blueprint/UI/UI_ItemTooltip.Update Item` _asui_item_tooltip (`self.ItemData`))
  (bind _asui_item_slot (cast `/Game/Blueprint/UI/UI_ItemSlot` (`WidgetComponent.GetUserWidgetObject` (`self.ItemSlotWidget`))))
  (`/Game/Blueprint/UI/UI_ItemSlot.UpdateItem` _asui_item_slot (`self.ItemData`)))

(fn `BeamFollowItem`
  (bind (_returnvalue_roll _returnvalue_pitch _returnvalue_yaw) (`KismetMathLibrary.BreakRotator` (`KismetMathLibrary.FindLookAtRotation` (`self.K2_GetActorLocation`) (`self.K2_GetActorLocation` (`self.CharRef`)))))
  (`SceneComponent.K2_SetWorldLocation` (`self.Beam`) (`SceneComponent.K2_GetComponentLocation` (`self.Box`)) false true)
  (if (`SceneComponent.IsVisible` (`self.ItemTooltipWidget`))
    (`SceneComponent.K2_SetWorldRotation` (`self.ItemTooltipWidget`) (`KismetMathLibrary.MakeRotator` 0.0 0.0 _returnvalue_yaw) false false)
    (`SceneComponent.K2_SetWorldRotation` (`self.ItemSlotWidget`) (`KismetMathLibrary.MakeRotator` 0.0 0.0 _returnvalue_yaw) false false)))

(fn `CheckPlayerRange`
  (`SceneComponent.SetVisibility` (`self.ItemTooltipWidget`) (<= (`self.GetDistanceTo` (`self.CharRef`)) 300.0) false)
  (`SceneComponent.SetVisibility` (`self.ItemSlotWidget`) (<= (`self.GetDistanceTo` (`self.CharRef`)) 300.0) false))

(fn `UserConstructionScript`)