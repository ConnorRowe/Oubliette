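; BP_Chest is an interactable chest that spawns a random item for the player to pick up.
; On BeginPlay it async-loads and attaches an inactive Niagara effect and randomly may swap to a cubic mesh.
; Interact sets ShouldOpen on a closed chest, or gives the spawned item to the character once open.
; OpenChest, not called here, activates the effect and spawns BP_Item from the GameMode's chest pool; selection toggles custom depth.
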(event `/Game/Blueprint/BPI_Interactable.Interact`
  (if (`self.isOpen`)
    (if (`self.itemExists`)
      (`/Game/Blueprint/Character/BP_Oubliette_Character.PickupItem` (`self.CharRef`) (`self.SpawnedItem`))
      (set `self.itemExists` false))
    (else
      (set `self.shouldOpen` true))))

(event `self.ReceiveBeginPlay`
  (set `self.CharRef` (cast `/Game/Blueprint/Character/BP_Oubliette_Character` (`GameInstanceOubliette.charRef` (cast `GameInstanceOubliette` (`GameplayStatics.GetGameInstance`) :!pure true)) :!pure true))
  (bind _object (`|LoadAsset` (`KismetSystemLibrary.Conv_SoftObjPathToSoftObjRef` (`self.NiagaraSystemAsset`)))
    (:`Completed`
      (bind _asniagara_system (cast `NiagaraSystem` _object))
      (bind _returnvalue (`NiagaraFunctionLibrary.SpawnSystemAttached` _asniagara_system (`self.ChestMesh`) "None" (-2.132678 0.0 32.231773) (struct) "KeepRelativeOffset"))
      (bind _output_get (set `self.NiagaraSystem` _returnvalue))
      (`ActorComponent.Deactivate` _output_get)
      (if (`KismetMathLibrary.RandomBool`)
        (`SkinnedMeshComponent.SetSkinnedAssetAndUpdate` (`self.ChestMesh`) "/Game/Meshes/Skeletal/SK_ChestCubic.SK_ChestCubic" false)))))

(event `/Game/Blueprint/BPI_Selectable.SelectObject`
  (params (isSelected :type Boolean))
  (`self.SetSelected` isSelected))

(fn `OpenChest`
  (bind (_returnvalue_location _returnvalue_rotation) (`KismetMathLibrary.BreakTransform` (`SceneComponent.K2_GetComponentToWorld` (`self.ItemLoc`))))
  (bind _asbp_game_mode_oubliette (cast `/Game/Blueprint/BP_GameModeOubliette` (`GameplayStatics.GetGameMode`) :!pure true))
  (`ActorComponent.Activate` (`self.NiagaraSystem`) false)
  (bind _returnvalue (`|SpawnActorFromClass` "/Game/Blueprint/Items/BP_Item.BP_Item_C" (`KismetMathLibrary.MakeTransform` _returnvalue_location _returnvalue_rotation) "AlwaysSpawn" "OverrideRootScale" null null))
  (bind _item (`/Game/Blueprint/BP_GameModeOubliette.GenerateRandomItem` _asbp_game_mode_oubliette (`GameModeOubliette.ItemPool_GeneralChest` _asbp_game_mode_oubliette)))
  (`/Game/Blueprint/Items/BP_Item.Init` _returnvalue _item)
  (set `self.SpawnedItem` _returnvalue)
  (set `self.itemExists` true))

(fn `SetSelected`
  (params (isSelected :type Boolean))
  (set `self.isSelected` isSelected)
  (`PrimitiveComponent.SetRenderCustomDepth` (`self.ChestMesh`) isSelected))

(fn `UserConstructionScript`)